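; BP_OverlapPlatform is a placeable moving platform that is triggered by overlap.
; Any component beginning overlap with its Box calls MovePlatform, with no filtering of the overlapping actor.
; On BeginPlay it binds a handler to the OnPlatformMoved dispatcher, which prints the platform's display name and whether it moved forward or backward, based on MovingForward.
; The movement logic itself is not defined in these graphs.
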(event OnComponentBeginOverlap(Box)
  (params (OverlappedComponent :type Primitive%20Component%20Object%20Reference) (OtherActor :type Actor%20Object%20Reference) (OtherComp :type Primitive%20Component%20Object%20Reference) (OtherBodyIndex :type Integer) (bFromSweep :type Boolean) (SweepResult :type Hit%20Result%20Structure%20%28by%20ref%29))
  (Class|BasePlatform|MovePlatform))

(event Custom|OnPlatformMovedEcho
  (bind _returnvalue (Utilities|GetDisplayName 0))
  (if (Variables|Default|GetbMovingForward)
    (Development|PrintString (Utilities|String|ToString(Text) (Utilities|Text|FormatText "{name} move forward" _returnvalue)))
    (else
      (Development|PrintString (Utilities|String|ToString(Text) (Utilities|Text|FormatText "{name} move backward" _returnvalue))))))

(event EventBeginPlay
  (EventDispatchers|AssignOnPlatformMoved (delegate Custom|OnPlatformMovedEcho)))

(fn ConstructionScript)